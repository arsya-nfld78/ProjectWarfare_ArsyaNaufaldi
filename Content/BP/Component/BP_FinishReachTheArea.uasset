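; Finish trigger component Blueprint that ends the game when the player reaches a target area during the "ReachTheArea" objective.
; The construction script sizes the TargetArea box from BoxSize.
; On the player's first overlap only, it finds the tagged BP_PointObjective and checks ObjectiveProgress.
; If true, it completes the objective, shows WBP_FinishGame, switches to UI-only input with the cursor, and pauses the game.
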(event `self.TargetArea.OnComponentBeginOverlap`
  (params (OverlappedComponent :type "PrimitiveComponent Object Reference") (OtherActor :type "Actor Object Reference") (OtherComp :type "PrimitiveComponent Object Reference") (OtherBodyIndex :type Integer) (bFromSweep :type Boolean) (SweepResult :type "HitResult Structure (by ref)"))
  (bind _returnvalue (`GameplayStatics.GetPlayerController` 0))
  (if (== OtherActor (`GameplayStatics.GetPlayerCharacter` 0))
    (`/Engine/EditorBlueprintResources/StandardMacros.DoOnce` false
      (:`Completed`
        (bind _outactors (`GameplayStatics.GetAllActorsOfClassWithTag` "/Game/BP/Component/BP_PointObjective.BP_PointObjective_C" "ReachTheArea"))
        (bind _output (`|GetArrayItem` _outactors))
        (if (`/Game/BP/Component/BP_PointObjective.ObjectiveProgress` _output)
          (`/Game/BP/Component/BP_PointObjective.ObjectiveComplete` _output)
          (bind _returnvalue_2 (`|CreateWidget` "/Game/UI/WBP_FinishGame.WBP_FinishGame_C"))
          (`UserWidget.AddToViewport` _returnvalue_2 0)
          (set `PlayerController.bShowMouseCursor` true _returnvalue)
          (`WidgetBlueprintLibrary.SetInputMode_UIOnlyEx` _returnvalue null)
          (`GameplayStatics.SetGamePaused` true))))))

(fn `UserConstructionScript`
  (`BoxComponent.SetBoxExtent` (`self.TargetArea`) (`self.BoxSize`) true))