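; BPC_Score is a component that tracks a score and shows it on the player's HUD.
; AddScore adds an amount to Score, while ReduceScore sets Score to the passed amount minus the current Score (not the reverse), clamped to zero or above.
; Both then call UpdateUIScore, which casts player character 0 to BP_Player and passes the score as text to its HUD widget's UpdateUI.
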(fn `AddScore`
  (params (AddScore :type Integer))
  (set `self.Score` (+ AddScore (`self.Score`)))
  (`self.UpdateUIScore`))

(fn `ReduceScore`
  (params (ReduceScore :type Integer))
  (set `self.Score` (`KismetMathLibrary.Clamp` (- ReduceScore (`self.Score`)) 0 2147483647))
  (`self.UpdateUIScore`))

(fn `UpdateUIScore`
  (bind _asbp_player (cast `/Game/ThirdPerson/Blueprints/Player/BP_Player` (`GameplayStatics.GetPlayerCharacter` 0)))
  (`/Game/UI/WBP_HUD.UpdateUI` (`/Game/ThirdPerson/Blueprints/Player/BP_Player.WBP_HUD_var` _asbp_player) (`KismetTextLibrary.Conv_IntToText` (`self.Score`))))