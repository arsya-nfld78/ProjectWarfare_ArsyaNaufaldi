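; BP_PointObjective is a trigger box that shows an on-screen objective when the player character enters it.
; BeginPlay creates a WBP_Objective widget, and the first player overlap fills in its title and content, adds it to the viewport and sets ObjectiveProgress.
; The ObjectiveComplete event changes the title to a completion message, dims the content and removes the widget after a short delay.
; The construction script sizes the box from BoxSize.
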(event `self.ReceiveBeginPlay`
  (bind _returnvalue (`|CreateWidget` "/Game/UI/WBP_Objective.WBP_Objective_C" null (`self.ObjectiveTitleTxt`) (`self.ObjectiveContentTxt`)))
  (set `self.WBP_Objective` _returnvalue))

(event `self.ObjectivePoint.OnComponentBeginOverlap`
  (params (OverlappedComponent :type "PrimitiveComponent Object Reference") (OtherActor :type "Actor Object Reference") (OtherComp :type "PrimitiveComponent Object Reference") (OtherBodyIndex :type Integer) (bFromSweep :type Boolean) (SweepResult :type "HitResult Structure (by ref)"))
  (bind _wbp_objective (`self.WBP_Objective`))
  (if (== OtherActor (`GameplayStatics.GetPlayerCharacter` 0))
    (`/Engine/EditorBlueprintResources/StandardMacros.DoOnce` false
      (:`Completed`
        (set `/Game/UI/WBP_Objective.Objective_Title_txt` (`self.ObjectiveTitleTxt`) _wbp_objective)
        (set `/Game/UI/WBP_Objective.Objective_Content_txt` (`self.ObjectiveContentTxt`) _wbp_objective)
        (`TextBlock.SetColorAndOpacity` (`/Game/UI/WBP_Objective.Objective_Content` _wbp_objective) (make `SlateColor` (struct :`R` 1.0 :`G` 1.0 :`B` 1.0 :`A` 1.0)))
        (`UserWidget.AddToViewport` (`self.WBP_Objective`) 0)
        (set `self.ObjectiveProgress` true)))))

(event `ObjectiveComplete`
  (bind _wbp_objective (`self.WBP_Objective`))
  (set `/Game/UI/WBP_Objective.Objective_Title_txt` "Objective Complete" _wbp_objective)
  (`TextBlock.SetColorAndOpacity` (`/Game/UI/WBP_Objective.Objective_Content` _wbp_objective) (make `SlateColor` (struct :`R` 1.0 :`G` 1.0 :`B` 1.0 :`A` 0.5)))
  (`KismetSystemLibrary.Delay` 2.0)
  (`Widget.RemoveFromParent` (`self.WBP_Objective`)))

(fn `UserConstructionScript`
  (`BoxComponent.SetBoxExtent` (`self.ObjectivePoint`) (`self.BoxSize`) true))