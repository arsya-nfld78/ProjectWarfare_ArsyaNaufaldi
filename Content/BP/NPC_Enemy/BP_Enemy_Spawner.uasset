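; BP_Enemy_Spawner spawns BP_Enemy_Insurgent1 enemies at its own location and rotation.
; SpawnEnemy loops to spawn a given count at once, adjusting for collision but always spawning.
; BatchSpawnEnemy calls it repeatedly with a Delay between batches.
; The batch counter subtracts zero, so batches repeat indefinitely whenever BatchCount is positive.
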(event `SpawnEnemy`
  (params (SpawnEnemyCount :type Integer))
  ;[1 1 1] Spawning Enemy Function
  (set `self.SpawnEnemyCount` SpawnEnemyCount)
  (while (> (`self.SpawnEnemyCount`) 0)
    (`|SpawnActorFromClass` "/Game/BP/NPC_Enemy/BP_Enemy_Insurgent1.BP_Enemy_Insurgent1_C" (`KismetMathLibrary.MakeTransform` (`self.K2_GetActorLocation`) (`self.K2_GetActorRotation`)) "AdjustIfPossibleButAlwaysSpawn" "MultiplyWithRoot" null null)
    (set `self.SpawnEnemyCount` (- (`self.SpawnEnemyCount`) 1))))

(event `BatchSpawnEnemy`
  (params (BatchCount :type Integer) (SpawnEnemyContPerBatch :type Integer) (Interval :type "Float (double-precision)"))
  ;[1 1 1] Batch Spawn Function
  (set `self.BatchCount` BatchCount)
  (`self.SpawnEnemy` SpawnEnemyContPerBatch :!label _label)
  (set `self.BatchCount` (- (`self.BatchCount`) 0))
  (`KismetSystemLibrary.Delay` Interval)
  (if (> (`self.BatchCount`) 0)
    (goto _label)))

(fn `UserConstructionScript`)