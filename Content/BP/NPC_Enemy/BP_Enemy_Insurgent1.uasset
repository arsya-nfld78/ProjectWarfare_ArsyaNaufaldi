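; Insurgent enemy NPC that roams random reachable points, chases any pawn it sees and shoots with a rifle.
; Pawn sensing drives the chase and fires when the move succeeds or fails, while a retriggerable delay resumes roaming after sightings stop.
; Firing plays a montage, then line-traces from the muzzle socket to apply damage, throttled by a resetting DoOnce.
; Incoming damage lowers health and enables mesh physics on death, without stopping the AI logic.
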(event `self.ReceiveBeginPlay`
  ;[1 1 1] Execution
  (set `CharacterMovementComponent.MaxWalkSpeed` 450.0 (`self.CharacterMovement`))
  (`self.Random roam`))

(event `Random roam`
  ;[1 1 1] Enemy Roamming/Patrolling
  (`|AIMoveTo` self (`NavigationSystemV1.K2_GetRandomReachablePointInRadius` (`self.K2_GetActorLocation`) 2500.0 null null) null
    (:`OnSuccess`
      (`self.Random roam`))))

(event `self.PawnSensing.OnSeePawn`
  (params (Pawn :type "Pawn Object Reference"))
  ;[1 1 1] Enemy Chase Player
  (`|ExecutionSequence`
    (:`then_0`
      (`|AIMoveTo` self (0.0 0.0 0.0) Pawn
        (:`OnSuccess`
          _)
        (:`OnFail`
          _))
      (`self.Fire`))
    (:`then_1`
      (`KismetSystemLibrary.RetriggerableDelay` 1.0)
      (`self.Random roam`))))

(event `Fire`
  (bind _returnvalue_location (`KismetMathLibrary.BreakTransform` (`SceneComponent.GetSocketTransform` (`self.Rifle`) "b_gun_muzzleflash" "RTS_World")))
  ;[1 1 1] Shoot Mechanic
  (`/Engine/EditorBlueprintResources/StandardMacros.DoOnce` false :!label _label
    (:`Completed`
      (`|ExecutionSequence`
        (:`then_0`
          (`|PlayMontage` (`self.Mesh`) "/Game/Characters/AnimationShooter/AS/AM/AM_Fire_Rifle_Ironsights.AM_Fire_Rifle_Ironsights"
            (:`then`
              (bind (_outhit _returnvalue) (`KismetSystemLibrary.LineTraceSingle` :`Start` _returnvalue_location :`End` (+ _returnvalue_location (* (`SceneComponent.GetRightVector` (`self.Mesh`)) 1000.0)) :`TraceChannel` "TraceTypeQuery1" :`DrawDebugType` "ForDuration" :`DrawTime` 2.0))
              (if _returnvalue
                (bind (_bblockinghit _binitialoverlap _time _distance _location _impactpoint _normal _impactnormal _physmat _hitactor) (`GameplayStatics.BreakHitResult` _outhit))
                (`KismetSystemLibrary.PrintString` (`KismetSystemLibrary.GetDisplayName` _hitactor))
                (`GameplayStatics.ApplyDamage` _hitactor 10.0)))))
        (:`then_1`
          (`KismetSystemLibrary.Delay` 0.1)
          (goto _label :!via `Reset`))))))

(event `self.ReceiveAnyDamage`
  (params (Damage :type "Float (single-precision)") (DamageType :type "DamageType Object Reference") (InstigatedBy :type "Controller Object Reference") (DamageCauser :type "Actor Object Reference"))
  ;[1 1 1] Shoot Mechanic
  ;;[1 1 1] Damage System
  (if (not (`self.IsDead`))
    (set `self.CurrentHealth` (- (`self.CurrentHealth`) Damage))
    (set `self.IsDead` (<= (`self.CurrentHealth`) 0.0))
    (`KismetSystemLibrary.PrintString` (`KismetStringLibrary.Conv_DoubleToString` (`self.CurrentHealth`)))
    (if (`self.IsDead`)
      (`PrimitiveComponent.SetSimulatePhysics` (`self.Mesh`) true))))

(fn `UserConstructionScript`)